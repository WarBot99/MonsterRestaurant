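; BP_StationBase is a base Blueprint for a minigame station that tracks when the first-person character is within interaction range.
; Overlapping the InteractionRange component sets UseRange and registers the station as InteractableToPick on the character's BasePlayerController.
; Leaving the range clears UseRange and resets InteractableToPick to None, without checking whether another station has since registered.
; The Blueprint contains no use logic of its own, and its construction script is empty.
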(event OnComponentBeginOverlap(InteractionRange)
  (params (OverlappedComponent :type Primitive%20Component%20Object%20Reference) (OtherActor :type Actor%20Object%20Reference) (OtherComp :type Primitive%20Component%20Object%20Reference) (OtherBodyIndex :type Integer) (bFromSweep :type Boolean) (SweepResult :type Hit%20Result%20Structure%20%28by%20ref%29))
  (bind _asbp_first_person_character (Utilities|Casting|CastToBP_FirstPersonCharacter OtherActor))
  (Variables|Default|SetUseRange true)
  (bind _asbase_player_controller (Utilities|Casting|CastToBasePlayerController (Pawn|GetController _asbp_first_person_character)))
  (Variables|/Game/FirstPerson/Blueprints/BasePlayerController.BasePlayerController_C|SetInteractableToPick _asbase_player_controller self))

(event OnComponentEndOverlap(InteractionRange)
  (params (OverlappedComponent :type Primitive%20Component%20Object%20Reference) (OtherActor :type Actor%20Object%20Reference) (OtherComp :type Primitive%20Component%20Object%20Reference) (OtherBodyIndex :type Integer))
  (bind _asbp_first_person_character (Utilities|Casting|CastToBP_FirstPersonCharacter OtherActor))
  (Variables|Default|SetUseRange false)
  (bind _asbase_player_controller (Utilities|Casting|CastToBasePlayerController (Pawn|GetController _asbp_first_person_character)))
  (Variables|/Game/FirstPerson/Blueprints/BasePlayerController.BasePlayerController_C|SetInteractableToPick _asbase_player_controller 0))

(fn ConstructionScript)